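; BP_NeonDashGameMode is the game mode Blueprint for Neon Dash, with no active logic in its graphs.
; BeginPlay and the construction script are empty.
; A disconnected chain would replace an existing controlled pawn with a BP_NeonDashPlayerPawn at a random spawn point and possess it.
; That unused chain would also set the view target to GameCamera and print the player count.
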(event EventBeginPlay)

(fn ConstructionScript)